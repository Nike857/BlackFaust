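; BP_juese_rifumei is a player-controlled character Blueprint with basic movement, camera look and jump through Enhanced Input.
; On BeginPlay it adds the Shuruyingsheqingjing01 mapping context to player 0's input subsystem.
; WASD input moves the character relative to control-rotation yaw, so pitch does not affect direction.
; Look input drives controller yaw and inverted, half-rate pitch, while Space starts and stops jumping.
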(event `self.ReceiveBeginPlay`
  (bind _returnvalue (pcsubsystem `EnhancedInputLocalPlayerSubsystem` (`GameplayStatics.GetPlayerController` 0)))
  (`/Engine/EditorBlueprintResources/StandardMacros.IsValid` _returnvalue
    (:`Is Valid`
      (`EnhancedInputSubsystemInterface.AddMappingContext` _returnvalue "/Game/rifumei/kongzhi/shuruyingsheqingjing01.shuruyingsheqingjing01" 0 (struct)))))

(event `EnhancedInput|/Game/rifumei/kongzhi/tiaoyue_kongge`
  (params (ActionValue :type Boolean) (ElapsedSeconds :type "Float (double-precision)") (TriggeredSeconds :type "Float (double-precision)") (InputAction :type "InputAction Object Reference" :default "/Game/rifumei/kongzhi/tiaoyue_kongge.tiaoyue_kongge"))
  (:`Started`
    (`self.Jump`))
  (:`Completed`
    (`self.StopJumping`)))

(event `EnhancedInput|/Game/rifumei/kongzhi/shijiao`
  (params (ActionValue :type "Vector2D Structure") (ElapsedSeconds :type "Float (double-precision)") (TriggeredSeconds :type "Float (double-precision)") (InputAction :type "InputAction Object Reference" :default "/Game/rifumei/kongzhi/shijiao.shijiao"))
  (:`Triggered`
    (`self.AddControllerYawInput` ActionValue_X)
    (`self.AddControllerPitchInput` (* ActionValue_Y -0.5))))

(event `EnhancedInput|/Game/rifumei/kongzhi/yidong_WASD`
  (params (ActionValue :type "Vector2D Structure") (ElapsedSeconds :type "Float (double-precision)") (TriggeredSeconds :type "Float (double-precision)") (InputAction :type "InputAction Object Reference" :default "/Game/rifumei/kongzhi/yidong_WASD.yidong_WASD"))
  (bind (_returnvalue_roll _returnvalue_pitch _returnvalue_yaw) (`KismetMathLibrary.BreakRotator` (`self.GetControlRotation`)))
  (:`Triggered`
    (`self.AddMovementInput` (`KismetMathLibrary.GetRightVector` (`KismetMathLibrary.MakeRotator` 0.0 0.0 _returnvalue_yaw)) ActionValue_X)
    (`self.AddMovementInput` (`KismetMathLibrary.GetForwardVector` (`KismetMathLibrary.MakeRotator` 0.0 0.0 _returnvalue_yaw)) ActionValue_Y)))

(fn `UserConstructionScript`)